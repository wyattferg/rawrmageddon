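; BP_Asteroid is an actor that moves through three staged positions.
; On BeginPlay a timeline lerps it from its starting location toward the stage one position with swept movement.
; Each NextStage event increments the stage counter, captures the current location and starts the timeline toward the stage two or three position.
; The newer timeline stops the previous one as it updates, so a stage change can interrupt movement underway.
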(event Custom|NextStage
  (Variables|Default|SetcurrentPos (Transformation|GetActorLocation))
  (bind _result (Math|Integer|IncrementInt (Variables|Default|GetcurrentStage))
    (:%20%20
      (switch int _result
        (:2
          (bind _newtrack_0 (Timeline|Timeline_0 PlayFromStart)
            (:Update
              (Transformation|SetActorLocation (Math|Vector|Lerp(Vector) (Variables|Default|GetcurrentPos) (Variables|Default|GetStageTwoPosition) _newtrack_0) true false)
              (bind _newtrack_0_2 (Timeline|Timeline Stop)
                (:Update
                  (Transformation|SetActorLocation (Math|Vector|Lerp(Vector) (Variables|Default|GetcurrentPos) (Variables|Default|GetStageOnePosition) _newtrack_0_2) true false))))))
        (:3
          (bind _newtrack_0_3 (Timeline|Timeline_1 PlayFromStart)
            (:Update
              (Transformation|SetActorLocation (Math|Vector|Lerp(Vector) (Variables|Default|GetcurrentPos) (Variables|Default|GetStageThreePosition) _newtrack_0_3) true false)
              (Timeline|Timeline_0 Stop))))))))

(event EventBeginPlay
  (Variables|Default|SetcurrentPos (Transformation|GetActorLocation))
  (bind _newtrack_0 (Timeline|Timeline PlayFromStart)
    (:Update
      (Transformation|SetActorLocation (Math|Vector|Lerp(Vector) (Variables|Default|GetcurrentPos) (Variables|Default|GetStageOnePosition) _newtrack_0) true false))))

(fn ConstructionScript)