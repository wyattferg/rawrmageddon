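; BP_SpeedRing is a speed boost ring that raises the third-person character's max walk speed when it enters the ring's box.
; Each boost multiplies the current walk speed, clamped to a fixed range, and increments the character's NumRingsActive counter.
; An IsUsing flag blocks retriggering until a short delay ends and decrements the counter.
; The ring itself never restores the walk speed.
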(event OnComponentBeginOverlap(Box)
  (params (OverlappedComponent :type Primitive%20Component%20Object%20Reference) (OtherActor :type Actor%20Object%20Reference) (OtherComp :type Primitive%20Component%20Object%20Reference) (OtherBodyIndex :type Integer) (bFromSweep :type Boolean) (SweepResult :type Hit%20Result%20Structure%20%28by%20ref%29))
  (if (not (Variables|Default|GetisUsing))
    (bind _asbp_third_person_character (Utilities|Casting|CastToBP_ThirdPersonCharacter OtherActor))
    (Variables|Default|SetisUsing true)
    (Variables|/Script/Engine.CharacterMovementComponent|SetMaxWalkSpeed (Variables|/Script/Engine.Character|GetCharacterMovement _asbp_third_person_character) (Math|Float|Clamp(Float) (* (Variables|/Script/Engine.CharacterMovementComponent|GetMaxWalkSpeed (Variables|/Script/Engine.Character|GetCharacterMovement _asbp_third_person_character)) 1.5) 6e+02 2.4e+03))
    (Math|Integer|IncrementInt (Variables|/Game/ThirdPerson/Blueprints/BP_ThirdPersonCharacter.BP_ThirdPersonCharacter_C|GetnumRingsActive _asbp_third_person_character)
      (:%20%20
        (Utilities|FlowControl|Delay 3.0)
        (Variables|Default|SetisUsing false)
        (Math|Integer|DecrementInt (Variables|/Game/ThirdPerson/Blueprints/BP_ThirdPersonCharacter.BP_ThirdPersonCharacter_C|GetnumRingsActive _asbp_third_person_character))))))

(fn ConstructionScript)