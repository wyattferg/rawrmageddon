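; BP_KillZone is a volume that kills the player character for leaving it.
; Half a second after BeginPlay it records whether a BP_ThirdPersonCharacter starts inside by checking overlapping actors.
; When an overlap ends and no character remains, it waits a second, rechecks, then calls PlayerDeath on the exiting actor and clears the inside flag.
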(event OnComponentEndOverlap(Box)
  (params (OverlappedComponent :type Primitive%20Component%20Object%20Reference) (OtherActor :type Actor%20Object%20Reference) (OtherComp :type Primitive%20Component%20Object%20Reference) (OtherBodyIndex :type Integer))
  (bind _overlappingactors (Collision|GetOverlappingActors "/Game/ThirdPerson/Blueprints/BP_ThirdPersonCharacter.BP_ThirdPersonCharacter_C" :!class /Script/Engine.Actor))
  (bind _returnvalue (Utilities|Array|IsEmpty _overlappingactors))
  (if (Variables|Default|GetisPlayerInside)
    (if _returnvalue
      (Utilities|FlowControl|Delay 1.0)
      (if _returnvalue
        (bind _asbp_third_person_character (Utilities|Casting|CastToBP_ThirdPersonCharacter OtherActor))
        (Default|PlayerDeath _asbp_third_person_character)
        (Variables|Default|SetisPlayerInside false)))))

(event Custom|StartPlayer
  (Utilities|FlowControl|Delay 0.5)
  (if (not (Utilities|Array|IsEmpty (Collision|GetOverlappingActors "/Game/ThirdPerson/Blueprints/BP_ThirdPersonCharacter.BP_ThirdPersonCharacter_C" :!class /Script/Engine.Actor)))
    (Variables|Default|SetisPlayerInside true)))

(event EventBeginPlay
  (CallFunction|StartPlayer))

(fn ConstructionScript)