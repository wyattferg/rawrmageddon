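; Game mode Blueprint that respawns the third-person player character through a RespawnPlayer event.
; The event flags the death, destroys the current character, then spawns and possesses a new one at the Checkpoint's spawn position, calling ConsistentTick on it.
; Without a valid checkpoint, it switches on level name to choose a hardcoded spawn transform.
; An out-of-lives return to the main menu exists but is disconnected.
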(event Custom|Respawn%20Player
  ;[0.15 0.15 0.15 0.5] Respawn Player
  (Variables|Default|SethasDied true)
  (Actor|DestroyActor (Game|GetPlayerCharacter 0))
  (Utilities|FlowControl|Sequence
    (:then_0
      (bind _checkpoint (Variables|Default|GetCheckpoint)
        (:then
          (bind _returnvalue (Game|SpawnActorfromClass "/Game/ThirdPerson/Blueprints/BP_ThirdPersonCharacter.BP_ThirdPersonCharacter_C" (Math|Transform|MakeTransform (.location (Transformation|GetWorldTransform (Variables|/Game/Blueprints/BP_Checkpoint.BP_Checkpoint_C|GetSpawn%20Position _checkpoint))) (.rotation (Transformation|GetWorldTransform (Variables|/Game/Blueprints/BP_Checkpoint.BP_Checkpoint_C|GetSpawn%20Position _checkpoint))) "1.000000,1.000000,1.000000") "AlwaysSpawn" "MultiplyWithRoot" 0 0))
          (Pawn|Possess (Game|GetPlayerController 0) _returnvalue)
          (Default|ConsistentTick _returnvalue))
        (:else
          (bind _returnvalue_2 (Game|GetCurrentLevelName true))
          (switch string _returnvalue_2
            (:Default
              (bind _returnvalue_3 (Game|SpawnActorfromClass "/Game/ThirdPerson/Blueprints/BP_ThirdPersonCharacter.BP_ThirdPersonCharacter_C" (Math|Transform|MakeTransform "0, 0, 0" "0, 0, 0" "1.000000,1.000000,1.000000") "Undefined" "MultiplyWithRoot" 0 0))
              (Pawn|Possess (Game|GetPlayerController 0) _returnvalue_3)
              (Default|ConsistentTick _returnvalue_3))
            (:PlaygroundMap
              (bind _returnvalue_4 (Game|SpawnActorfromClass "/Game/ThirdPerson/Blueprints/BP_ThirdPersonCharacter.BP_ThirdPersonCharacter_C" (Math|Transform|MakeTransform "-30.520647,894.428822,136.361132" "0, 0, 0" "1.000000,1.000000,1.000000") "Undefined" "MultiplyWithRoot" 0 0 :!label _label))
              (Pawn|Possess (Game|GetPlayerController 0) _returnvalue_4)
              (Default|ConsistentTick _returnvalue_4))
            (:Untitled
              (goto _label))
            (:Level1
              (bind _returnvalue_5 (Game|SpawnActorfromClass "/Game/ThirdPerson/Blueprints/BP_ThirdPersonCharacter.BP_ThirdPersonCharacter_C" (Math|Transform|MakeTransform "-506.931085,801315.928455,-28953.987220" "0, 0, 0" "1.000000,1.000000,1.000000") "Undefined" "MultiplyWithRoot" 0 0))
              (Pawn|Possess (Game|GetPlayerController 0) _returnvalue_5)
              (Default|ConsistentTick _returnvalue_5))
            (:Finale
              (bind _returnvalue_6 (Game|SpawnActorfromClass "/Game/ThirdPerson/Blueprints/BP_ThirdPersonCharacter.BP_ThirdPersonCharacter_C" (Math|Transform|MakeTransform "2307.877541,803595.271779,735.906573" "-29.345495,-879.270849,-108.436928" "1.000000,1.000000,1.000000") "Undefined" "MultiplyWithRoot" 0 0))
              (Pawn|Possess (Game|GetPlayerController 0) _returnvalue_6)
              (Default|ConsistentTick _returnvalue_6))))))))

(fn ConstructionScript)