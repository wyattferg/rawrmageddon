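; BP_Checkpoint is a trigger-based checkpoint that currently ends the level when the player character reaches it.
; On trigger overlap, if LevelPassed is true and the checkpoint is not already the game mode's LastCheckpoint, it records itself there.
; It then prints a message, opens the level menu map, shows the mouse cursor and switches input to UI only, an ending marked as temporary.
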(event OnComponentBeginOverlap(Trigger)
  (params (OverlappedComponent :type Primitive%20Component%20Object%20Reference) (OtherActor :type Actor%20Object%20Reference) (OtherComp :type Primitive%20Component%20Object%20Reference) (OtherBodyIndex :type Integer) (bFromSweep :type Boolean) (SweepResult :type Hit%20Result%20Structure%20%28by%20ref%29))
  (bind _returnvalue (Game|GetPlayerController 0))
  (bind _self self)
  ;[0.15 0.15 0.15 0.5] Set Checkpoint
  (if (Variables|Default|GetLevelPassed)
    (Utilities|Casting|CastToBP_ThirdPersonCharacter OtherActor)
    (bind _asbp_third_person_game_mode (Utilities|Casting|CastToBP_ThirdPersonGameMode (Game|GetGameMode)))
    (if (not (== (Variables|/Game/ThirdPerson/Blueprints/BP_ThirdPersonGameMode.BP_ThirdPersonGameMode_C|GetLast%20Checkpoint _asbp_third_person_game_mode) _self))
      (Variables|/Game/ThirdPerson/Blueprints/BP_ThirdPersonGameMode.BP_ThirdPersonGameMode_C|SetLast%20Checkpoint _asbp_third_person_game_mode _self)
      (Development|PrintString "Checkpoint Hit")
      ;[0.15 0 0 0.5] Once checkpoint reached, end level (for now)
      (Game|OpenLevel(byName) "levelmenumap")
      (Variables|/Script/Engine.PlayerController|SetbShowMouseCursor _returnvalue true)
      (Input|SetInputModeUIOnly _returnvalue 0 "DoNotLock" false))))

(event EventBeginPlay)

(event Collision|EventActorBeginOverlap
  (params (OtherActor :type Actor%20Object%20Reference)))

(event EventTick
  (params (DeltaSeconds :type Float%20%28single-precision%29)))

(fn ConstructionScript)