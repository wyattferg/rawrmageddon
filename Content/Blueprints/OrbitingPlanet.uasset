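; Orbiting planet actor that circles a pivot through its RotatingMovement component.
; On BeginPlay it attaches to ParentPlanet's static mesh when one is valid, keeping its world transform.
; It derives the rotation rate from TimeToComplete for one full revolution.
; The pivot offset is the negated world location, which targets the world origin for an unrotated actor rather than reading the parent's position.
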(event EventBeginPlay
  (bind _parentplanet (Variables|Default|GetParentPlanet))
  (bind _rotatingmovement (Variables|Default|GetRotatingMovement))
  (Utilities|IsValid _parentplanet
    (:Is%20Valid
      (Transformation|AttachComponentToComponent (Variables|/Script/Engine.StaticMeshActor|GetStaticMeshComponent _parentplanet) "None" "KeepWorld" "KeepWorld" "KeepWorld" false))
    (:Is%20Not%20Valid
      _))
  (Variables|/Script/Engine.RotatingMovementComponent|SetRotationRate _rotatingmovement (Math|Rotator|MakeRotator 0.0 0.0 (/ 3.6e+02 (Variables|Default|GetTimeToComplete))))
  (Variables|/Script/Engine.RotatingMovementComponent|SetPivotTranslation _rotatingmovement (Math|Vector|NegateVector (Transformation|GetActorLocation self))))

(fn ConstructionScript)