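; Item drop-off spot that shows a placed item as a constantly spinning mesh.
; DisplayInteract assigns the supplied mesh to the Item component and marks ObjectPlaced.
; Until then, BP_ThirdPersonCharacter entering the Trigger gets an on-screen hint that something belongs here.
; A level-specific step that sets the Checkpoint's LevelPassed is present but disconnected, so it never runs.
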(event OnComponentBeginOverlap(Trigger)
  (params (OverlappedComponent :type Primitive%20Component%20Object%20Reference) (OtherActor :type Actor%20Object%20Reference) (OtherComp :type Primitive%20Component%20Object%20Reference) (OtherBodyIndex :type Integer) (bFromSweep :type Boolean) (SweepResult :type Hit%20Result%20Structure%20%28by%20ref%29))
  ;[0.15 0.15 0.15 0.5] Detect If Player In Hitbox Range
  (if (not (Variables|Default|GetObjectPlaced))
    (bind _asbp_third_person_character (Utilities|Casting|CastToBP_ThirdPersonCharacter OtherActor))
    (Default|ScreenOutput _asbp_third_person_character "It looks like I should put something on this...")))

(event EventBeginPlay)

(event Collision|EventActorBeginOverlap
  (params (OtherActor :type Actor%20Object%20Reference)))

(event EventTick
  (params (DeltaSeconds :type Float%20%28single-precision%29))
  ;[0.15 0.15 0.15 0.5] Spin Item
  (Transformation|AddLocalRotation (Variables|Default|GetItem) "0.000000,0.500000,0.000000" false false))

(event EventDisplayInteract
  (params (Item :type Static%20Mesh%20Object%20Reference))
  ;[0.15 0.15 0.15 0.5] Display Item
  (Components|StaticMesh|SetStaticMesh (Variables|Default|GetItem) Item)
  (Variables|Default|SetObjectPlaced true))

(fn ConstructionScript)