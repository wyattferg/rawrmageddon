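; BP_Switch is an interactable switch that operates either a linked door or a linked spot light.
; On interaction, a valid DoorSelect takes priority and opens through its OpenDoorWithButton call.
; Otherwise a valid LightSelect toggles via the IsLightOn flag, switching its spot light intensity on or off.
; Each action prints a debug string to the screen.
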(event EventSwitchInteract
  (bind _lightselect (Variables|Default|GetLightSelect))
  (bind _spotlightcomponent (Variables|/Script/Engine.SpotLight|GetSpotLightComponent _lightselect))
  ;[0.15 0.15 0.15 0.5] Door Switch
  (if (Utilities|IsValid (Variables|Default|GetDoorSelect))
    (Default|OpenDoorwithButton (Variables|Default|GetDoorSelect) false)
    (Development|PrintString "Door Opened")
    (else
      ;[0.15 0.15 0.15 0.5] Light Switch
      (if (Utilities|IsValid (Variables|Default|GetLightSelect))
        (if (not (Variables|Default|GetIsLightOn))
          (Variables|Default|SetIsLightOn true)
          (Development|PrintString "Turn Light On")
          (Rendering|Components|Light|SetIntensity _spotlightcomponent 1e+02)
          (else
            (Variables|Default|SetIsLightOn false)
            (Development|PrintString "Turn Light Off")
            (Rendering|Components|Light|SetIntensity _spotlightcomponent 0.0)))))))

(fn ConstructionScript)