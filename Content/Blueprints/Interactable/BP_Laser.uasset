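; Repairable laser that the player fixes by placing crystals in three trigger slots, after which it fires at an asteroid.
; Empty slots show camera-facing prompts, and placing a crystal reveals its mesh and clears the player's held item.
; Once all three are placed, a timeline straightens the joint and aims it at the asteroid.
; Tick then keeps it aimed, calls LaserActivated on the player and stretches the beam to the target.
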(event Custom|OnRepaired
  (bind _joint (Variables|Default|GetJoint))
  (bind _newtrack_0 (Timeline|Timeline PlayFromStart)
    (:Update
      (Transformation|SetRelativeRotation (Variables|Default|GetJoint1) (Math|Rotator|MakeRotator (Math|Float|Lerp 4e+01 0.0 _newtrack_0) 0.0 0.0) false false)
      (Transformation|SetWorldRotation (Variables|Default|GetJoint) (Math|Rotator|Lerp(Rotator) (Transformation|GetWorldRotation _joint) (Math|Rotator|FindLookatRotation (Transformation|GetWorldLocation _joint) (Transformation|GetActorLocation (Variables|Default|Getasteroid))) _newtrack_0) false false))
    (:Finished
      (Variables|Default|SetisRepaired true))))

(event Custom|PlaceCrystal
  (if (Collision|IsOverlappingActor (Variables|Default|GetTrigger1) (Game|GetPlayerCharacter 0) :!class /Script/Engine.PrimitiveComponent)
    (if (not (Variables|Default|GethasCrystal1))
      (Rendering|SetVisibility (Variables|Default|GetCrystal1) true false)
      (Variables|Default|SethasCrystal1 true)
      (CallFunction|HideInteractPrompt :!label _label)
      (bind _asbp_third_person_character (Utilities|Casting|CastToBP_ThirdPersonCharacter (Game|GetPlayerCharacter 0)))
      (bind _output_get (Variables|/Game/ThirdPerson/Blueprints/BP_ThirdPersonCharacter.BP_ThirdPersonCharacter_C|SetCurrentItem _asbp_third_person_character 0))
      (Components|StaticMesh|SetStaticMesh (Variables|/Game/ThirdPerson/Blueprints/BP_ThirdPersonCharacter.BP_ThirdPersonCharacter_C|GetEquippedItem _asbp_third_person_character) _output_get)
      (if (Math|Boolean|ANDBoolean (Variables|Default|GethasCrystal1) (Variables|Default|GethasCrystal2) (Variables|Default|GethasCrystal3))
        (CallFunction|OnRepaired)))
    (elif (Collision|IsOverlappingActor (Variables|Default|GetTrigger2) (Game|GetPlayerCharacter 0) :!class /Script/Engine.PrimitiveComponent)
      (if (not (Variables|Default|GethasCrystal2))
        (Rendering|SetVisibility (Variables|Default|GetCrystal2) true false)
        (Variables|Default|SethasCrystal2 true)
        (goto _label))
      (elif (Collision|IsOverlappingActor (Variables|Default|GetTrigger3) (Game|GetPlayerCharacter 0) :!class /Script/Engine.PrimitiveComponent)
        (if (not (Variables|Default|GethasCrystal3))
          (Rendering|SetVisibility (Variables|Default|GetCrystal3) true false)
          (Variables|Default|SethasCrystal3 true)
          (goto _label))))))

(event EventShowInteractPrompt
  (if (Collision|IsOverlappingActor (Variables|Default|GetTrigger1) (Game|GetPlayerCharacter 0) :!class /Script/Engine.PrimitiveComponent)
    (if (not (Variables|Default|GethasCrystal1))
      (Rendering|SetVisibility (Variables|Default|GetTextRender1) true false))
    (elif (Collision|IsOverlappingActor (Variables|Default|GetTrigger2) (Game|GetPlayerCharacter 0) :!class /Script/Engine.PrimitiveComponent)
      (if (not (Variables|Default|GethasCrystal2))
        (Rendering|SetVisibility (Variables|Default|GetTextRender2) true false))
      (elif (Collision|IsOverlappingActor (Variables|Default|GetTrigger3) (Game|GetPlayerCharacter 0) :!class /Script/Engine.PrimitiveComponent)
        (if (not (Variables|Default|GethasCrystal3))
          (Rendering|SetVisibility (Variables|Default|GetTextRender3) true false))))))

(event EventHideInteractPrompt
  (Rendering|SetVisibility (Variables|Default|GetTextRender1) false false)
  (Rendering|SetVisibility (Variables|Default|GetTextRender2) false false)
  (Rendering|SetVisibility (Variables|Default|GetTextRender3) false false))

(event EventTick
  (params (DeltaSeconds :type Float%20%28single-precision%29))
  (bind _bulletparent (Variables|Default|GetBulletParent))
  (bind _relativescale3d (Variables|/Script/Engine.SceneComponent|GetRelativeScale3D _bulletparent))
  (if (Variables|Default|GetisRepaired)
    (Transformation|SetWorldRotation (Variables|Default|GetJoint) (Math|Rotator|FindLookatRotation (Transformation|GetWorldLocation (Variables|Default|GetJoint)) (Transformation|GetActorLocation (Variables|Default|Getasteroid))) false false)
    (bind _asbp_third_person_character (Utilities|Casting|CastToBP_ThirdPersonCharacter (Game|GetPlayerCharacter 0)))
    (Default|LaserActivated _asbp_third_person_character)
    (bind _newtrack_0 (Timeline|Timeline_0 PlayFromStart)
      (:Update
        (Transformation|SetRelativeScale3D _bulletparent (Math|Vector|Lerp(Vector) (Math|Vector|MakeVector (.x _relativescale3d) (.y _relativescale3d) (.z _relativescale3d)) (Math|Vector|MakeVector (.x _relativescale3d) (Math|Vector|Distance(Vector) (Transformation|GetWorldLocation _bulletparent) (Transformation|GetWorldLocation (Variables|/Game/Blueprints/BP_Asteroid.BP_Asteroid_C|Getasteroid_01 (Variables|Default|Getasteroid)))) (.z _relativescale3d)) _newtrack_0))))
    (else
      (if (Variables|Default|GethasCrystal1)
        _
        (else
          (Transformation|SetWorldRotation (Variables|Default|GetTextRender1) (Math|Rotator|FindLookatRotation (Transformation|GetWorldLocation (Variables|Default|GetTextRender1)) (Camera|GetCameraLocation (Game|GetPlayerCameraManager 0))) false false)))
      (if (Variables|Default|GethasCrystal2)
        _
        (else
          (Transformation|SetWorldRotation (Variables|Default|GetTextRender2) (Math|Rotator|FindLookatRotation (Transformation|GetWorldLocation (Variables|Default|GetTextRender2)) (Camera|GetCameraLocation (Game|GetPlayerCameraManager 0))) false false)))
      (if (not (Variables|Default|GethasCrystal3))
        (Transformation|SetWorldRotation (Variables|Default|GetTextRender3) (Math|Rotator|FindLookatRotation (Transformation|GetWorldLocation (Variables|Default|GetTextRender3)) (Camera|GetCameraLocation (Game|GetPlayerCameraManager 0))) false false)))))

(fn ConstructionScript
  (if (Variables|Default|GethasCrystal1)
    _
    (else
      (Rendering|SetVisibility (Variables|Default|GetCrystal1) false false)
      (Transformation|SetRelativeRotation (Variables|Default|GetJoint1) "0.000000,0.000000,40.000000" false false)
      (Variables|Default|SetisRepaired false)))
  (if (Variables|Default|GethasCrystal2)
    _
    (else
      (Rendering|SetVisibility (Variables|Default|GetCrystal2) false false)
      (Transformation|SetRelativeRotation (Variables|Default|GetJoint1) "0.000000,0.000000,40.000000" false false)
      (Variables|Default|SetisRepaired false)))
  (if (not (Variables|Default|GethasCrystal3))
    (Rendering|SetVisibility (Variables|Default|GetCrystal3) false false)
    (Transformation|SetRelativeRotation (Variables|Default|GetJoint1) "0.000000,0.000000,40.000000" false false)
    (Variables|Default|SetisRepaired false)))