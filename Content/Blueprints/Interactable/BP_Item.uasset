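; BP_Item is an interactable pickup item with a floating text prompt.
; The construction script applies the chosen mesh to the item model, and Tick turns the text to face the player camera.
; Show and hide events toggle the prompt's visibility.
; PickUp plays a timeline that shrinks the root to zero scale, then destroys the actor.
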(event EventBeginPlay)

(event Collision|EventActorBeginOverlap
  (params (OtherActor :type Actor%20Object%20Reference)))

(event EventTick
  (params (DeltaSeconds :type Float%20%28single-precision%29))
  (Transformation|SetWorldRotation (Variables|Default|GetTextRender) (Math|Rotator|FindLookatRotation (Transformation|GetWorldLocation (Variables|Default|GetTextRender)) (Camera|GetCameraLocation (Game|GetPlayerCameraManager 0))) false false))

(event EventShowInteractPrompt
  (Rendering|SetVisibility (Variables|Default|GetTextRender) true false))

(event EventPickUp
  ;[0.15 0.15 0.15 0.5] Destroy Item When Picked Up
  (bind _shrinktimeline (Timeline|Shrink Play)
    (:Update
      (Transformation|SetWorldScale3D (Variables|Default|GetDefaultSceneRoot) (Math|Conversions|ToVector(Float) (Math|Float|Lerp 1.0 0.0 _shrinktimeline))))
    (:Finished
      (Actor|DestroyActor))))

(event EventHideInteractPrompt
  (Rendering|SetVisibility (Variables|Default|GetTextRender) false false))

(fn ConstructionScript
  (Components|StaticMesh|SetStaticMesh (Variables|Default|GetItemModel) (Variables|Default|GetItemModelToPlace)))