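; BP_ItemDropOff is an interactable drop-off spot that displays a placed item as a slowly rotating static mesh.
; DisplayInteract stores and shows an incoming mesh, while DisplayItemPickUp clears it and returns it, with IsObjectPlaced tracking occupancy.
; The construction script shows any preset CurrentItem.
; Show and hide events toggle a text prompt that Tick turns toward the player camera; checkpoint-passing logic is present but unconnected.
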(event EventBeginPlay)

(event Collision|EventActorBeginOverlap
  (params (OtherActor :type Actor%20Object%20Reference)))

(event EventTick
  (params (DeltaSeconds :type Float%20%28single-precision%29))
  ;[0.15 0.15 0.15 0.5] Spin Item
  (Transformation|AddLocalRotation (Variables|Default|GetItem) "0.500000,0.500000,0.000000" false false)
  (Transformation|SetWorldRotation (Variables|Default|GetTextRender) (Math|Rotator|FindLookatRotation (Transformation|GetWorldLocation (Variables|Default|GetTextRender)) (Camera|GetCameraLocation (Game|GetPlayerCameraManager 0))) false false))

(event EventShowInteractPrompt
  (Rendering|SetVisibility (Variables|Default|GetTextRender) true false))

(event EventHideInteractPrompt
  (Rendering|SetVisibility (Variables|Default|GetTextRender) false false))

(event EventDisplayInteract
  (params (Item :type Static%20Mesh%20Object%20Reference))
  ;[0.15 0.15 0.15 0.5] Display Item
  (Components|StaticMesh|SetStaticMesh (Variables|Default|GetItem) Item)
  (Variables|Default|SetCurrentItem Item)
  (Variables|Default|SetIsObjectPlaced true))

(fn ConstructionScript
  (bind _currentitem (Variables|Default|GetCurrentItem))
  (Utilities|IsValid _currentitem
    (:Is%20Valid
      (Components|StaticMesh|SetStaticMesh (Variables|Default|GetItem) _currentitem)
      (Variables|Default|SetIsObjectPlaced true))))

(fn DisplayItemPickUp
  (Components|StaticMesh|SetStaticMesh (Variables|Default|GetItem) 0)
  (bind _output_get (LocalVariables|SetItemRef (Variables|Default|GetCurrentItem)))
  (Variables|Default|SetCurrentItem 0)
  (Variables|Default|SetIsObjectPlaced false)
  (return _output_get))