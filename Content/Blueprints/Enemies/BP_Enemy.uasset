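; BP_Enemy is an enemy character that chases the player within range and, up close, lunges to deal damage after a random delay.
; Tick points gravity toward the last overlapped TriggerSphere and drives movement, attacks and ragdoll death before destruction.
; Ground-pound radial damage and headbutts reduce health, launch it away and against gravity, and trigger an impact and material flash.
; A GameMode hitstop event briefly lowers custom time dilation.
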(event Custom|HeadbuttDamage
  (bind _mesh (Variables|Character|GetMesh))
  ;[0.15 0.15 0.15 0.5] Headbutt Damage
  (Math|Float|CompareFloat (Variables|Default|GetHealth) 0.0
    (:>
      (Variables|Default|SetHealth (- (Variables|Default|GetHealth) 1.0))
      (Character|LaunchCharacter (* (+ (Math|Vector|Normalize (Math|Vector|GetUnitDirection(Vector) (Transformation|GetActorLocation (Game|GetPlayerCharacter 0)) (Transformation|GetActorLocation))) (Math|Vector|NegateVector (Class|CharacterMovementComponent|GetGravityDirection (Variables|Character|GetCharacterMovement)))) 1e+03) false false)
      ;[0.15 0.15 0.15 0.5] Enemy Reaction to Damage
      (Game|SpawnActorfromClass "/Game/Blueprints/BP_Impact.BP_Impact_C" (Math|Transform|MakeTransform (Transformation|GetActorLocation) "0, 0, 0" "1.000000,1.000000,1.000000") "Undefined" "MultiplyWithRoot" 0 0)
      (Rendering|Material|SetMaterial _mesh 0 "/Game/LevelPrototyping/Materials/M_DamageFlash.M_DamageFlash")
      (Rendering|Material|SetMaterial _mesh 1 "/Game/LevelPrototyping/Materials/M_DamageFlash.M_DamageFlash")
      (Utilities|FlowControl|Delay 0.2)
      (Rendering|Material|SetMaterial _mesh 0 "/Game/Characters/Mannequins/Materials/Instances/Quinn/MI_Quinn_01.MI_Quinn_01")
      (Rendering|Material|SetMaterial _mesh 1 "/Game/Characters/Mannequins/Materials/Instances/Quinn/MI_Quinn_02.MI_Quinn_02"))))

(event Custom|On%20Hitstop
  (params (Time :type Float%20%28double-precision%29) (Weight :type Float%20%28double-precision%29) (Multiplier :type Float%20%28double-precision%29))
  ;[0.15 0.15 0.15 0.5] Hitstop Effect
  (bind _outactors (Actor|GetAllActorsOfClass "BP_Enemy_C"))
  (for _array_element _outactors
    (Variables|Default|SetCustomTimeDilation 0.1))
  (Utilities|FlowControl|Delay (* Time Weight Multiplier))
  (for _array_element_2 _outactors
    (Variables|Default|SetCustomTimeDilation 1.0)))

(event Game|Damage|EventRadialDamage
  (params (DamageReceived :type Float%20%28single-precision%29) (DamageType :type Damage%20Type%20Object%20Reference) (Origin :type Vector :default "0, 0, 0") (HitInfo :type Hit%20Result%20Structure%20%28by%20ref%29) (InstigatedBy :type Controller%20Object%20Reference) (DamageCauser :type Actor%20Object%20Reference))
  (bind _returnvalue (Transformation|GetActorLocation))
  (bind _mesh (Variables|Character|GetMesh))
  ;[0.15 0.15 0.15 0.5] Kickback from Ground Pound
  (Math|Float|CompareFloat (Variables|Default|GetHealth) 0.0
    (:>
      (Variables|Default|SetHealth (- (Variables|Default|GetHealth) DamageReceived))
      (Character|LaunchCharacter (* (* DamageReceived 6e+02) (+ (Math|Vector|Normalize (Math|Vector|GetUnitDirection(Vector) Origin _returnvalue)) (Math|Vector|NegateVector (Class|CharacterMovementComponent|GetGravityDirection (Variables|Character|GetCharacterMovement))))) false false)
      ;[0.15 0.15 0.15 0.5] Enemy Reaction to Damage
      (Game|SpawnActorfromClass "/Game/Blueprints/BP_Impact.BP_Impact_C" (Math|Transform|MakeTransform _returnvalue "0, 0, 0" "1.000000,1.000000,1.000000") "Undefined" "MultiplyWithRoot" 0 0)
      (Rendering|Material|SetMaterial _mesh 0 "/Game/LevelPrototyping/Materials/M_DamageFlash.M_DamageFlash")
      (Rendering|Material|SetMaterial _mesh 1 "/Game/LevelPrototyping/Materials/M_DamageFlash.M_DamageFlash")
      (Utilities|FlowControl|Delay 0.2)
      (Rendering|Material|SetMaterial _mesh 0 "/Game/Characters/Mannequins/Materials/Instances/Quinn/MI_Quinn_01.MI_Quinn_01")
      (Rendering|Material|SetMaterial _mesh 1 "/Game/Characters/Mannequins/Materials/Instances/Quinn/MI_Quinn_02.MI_Quinn_02"))))

(event EventBeginPlay
  (bind _asbp_game_mode (Utilities|Casting|CastToBP_GameMode (Game|GetGameMode)))
  (EventDispatchers|BindEventtoOnHitstop _asbp_game_mode (EventDispatchers|CreateEvent :!event Custom|On%20Hitstop)))

(event EventTick
  (params (DeltaSeconds :type Float%20%28single-precision%29))
  (bind _returnvalue (Game|GetPlayerCharacter 0))
  (bind _overlappingactors (Collision|GetOverlappingActors "/Script/Engine.TriggerSphere" :!class /Script/Engine.Actor))
  (bind _returnvalue_2 (Transformation|GetActorLocation))
  (bind _returnvalue_3 (Game|GetPlayerCharacter 0))
  (bind _mesh (Variables|Character|GetMesh))
  (bind _attackdistance (Variables|Default|GetAttackDistance))
  (bind _returnvalue_4 (Utilities|Array|Length _overlappingactors))
  (bind _returnvalue_5 (Transformation|GetActorLocation _returnvalue))
  (bind _returnvalue_6 (Math|Vector|Distance(Vector) _returnvalue_5 _returnvalue_2))
  (bind _returnvalue_7 (>= _returnvalue_6 _attackdistance))
  ;[0.15 0.15 0.15 0.5] Gravity Control
  (if (== _returnvalue_4 0)
    (Class|CharacterMovementComponent|SetGravityDirection (Variables|Character|GetCharacterMovement) (Math|Vector|MakeVector 0.0 0.0 0.0))
    (else
      (Class|CharacterMovementComponent|SetGravityDirection (Variables|Character|GetCharacterMovement) (Math|Vector|Normalize (- (Transformation|GetActorLocation (Utilities|Array|Get(acopy) _overlappingactors (- _returnvalue_4 1))) (Transformation|GetActorLocation))))))
  (Math|Float|CompareFloat (Variables|Default|GetHealth) 0.0
    (:>
      ;[0.15 0.15 0.15 0.5] Movement Control
      ;;[0.15 0.15 0.15 0.5] If too close, attack
      (if _returnvalue_7
        ;;[0.15 0 0 0.5] If too far, wander (inactive)
        (if (< _returnvalue_6 (Variables|Default|GetWanderDistance)) :!label _label
          ;;[0.15 0.15 0.15 0.5] If within range, go to player
          (Pawn|Input|AddMovementInput (Math|Vector|Normalize (- _returnvalue_5 _returnvalue_2)) 0.7 false))
        (else
          (Utilities|FlowControl|Delay (Math|Random|RandomFloatinRange 0.0 3.0))
          (if _returnvalue_7
            (goto _label)
            (else
              (Character|LaunchCharacter (* (Math|Vector|Normalize (Math|Vector|GetUnitDirection(Vector) (Transformation|GetActorLocation) (Transformation|GetActorLocation _returnvalue_3))) 1e+03) false false)
              (Game|Damage|ApplyDamage _returnvalue_3 1.0 0 self))))))
    (:==
      ;[0.15 0.15 0.15 0.5] Death
      (Physics|SetSimulatePhysics (Variables|Character|GetMesh) true :!label _label_2)
      (Physics|SetSimulatePhysics (Variables|Default|GetCapsuleComponent) true)
      (Collision|SetCollisionProfileName (Variables|Character|GetMesh) "BlockAll" true :!class /Script/Engine.PrimitiveComponent)
      (Collision|SetCollisionResponsetoChannel _mesh "ECC_Pawn" "ECR_Ignore")
      (Collision|SetCollisionResponsetoChannel _mesh "ECC_Visibility" "ECR_Ignore")
      (Utilities|FlowControl|Delay 3.0)
      (Actor|DestroyActor))
    (:<
      (goto _label_2))))

(fn ConstructionScript)