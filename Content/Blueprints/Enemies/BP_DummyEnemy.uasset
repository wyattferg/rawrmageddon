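; BP_DummyEnemy is a test-dummy style enemy that follows custom gravity and visibly reacts to being hit.
; Each tick it points CharacterMovement gravity toward the last actor overlapping TriggerSphere, or passes a zero vector when none overlap.
; Tail attack and radial damage events share one reaction that spawns BP_Impact and briefly swaps both mesh materials to a damage flash, with no health handling.
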(event Custom|Tail%20Attack%20Damage
  (bind _mesh (Variables|Character|GetMesh))
  ;[0.15 0.15 0.15 0.5] Enemy Reaction to Damage
  (Game|SpawnActorfromClass "/Game/Blueprints/BP_Impact.BP_Impact_C" (Math|Transform|MakeTransform (Transformation|GetActorLocation) "0, 0, 0" "1.000000,1.000000,1.000000") "Undefined" "MultiplyWithRoot" 0 0)
  (Rendering|Material|SetMaterial _mesh 0 "/Game/LevelPrototyping/Materials/M_DamageFlash.M_DamageFlash")
  (Rendering|Material|SetMaterial _mesh 1 "/Game/LevelPrototyping/Materials/M_DamageFlash.M_DamageFlash")
  (Utilities|FlowControl|Delay 0.2)
  (Rendering|Material|SetMaterial _mesh 0 "/Game/Characters/Mannequins/Materials/Instances/Quinn/MI_Quinn_01.MI_Quinn_01")
  (Rendering|Material|SetMaterial _mesh 1 "/Game/Characters/Mannequins/Materials/Instances/Quinn/MI_Quinn_02.MI_Quinn_02"))

(event Game|Damage|EventRadialDamage
  (params (DamageReceived :type Float%20%28single-precision%29) (DamageType :type Damage%20Type%20Object%20Reference) (Origin :type Vector :default "0, 0, 0") (HitInfo :type Hit%20Result%20Structure%20%28by%20ref%29) (InstigatedBy :type Controller%20Object%20Reference) (DamageCauser :type Actor%20Object%20Reference))
  (bind _mesh (Variables|Character|GetMesh))
  ;[0.15 0.15 0.15 0.5] Enemy Reaction to Damage
  (Game|SpawnActorfromClass "/Game/Blueprints/BP_Impact.BP_Impact_C" (Math|Transform|MakeTransform (Transformation|GetActorLocation) "0, 0, 0" "1.000000,1.000000,1.000000") "Undefined" "MultiplyWithRoot" 0 0)
  (Rendering|Material|SetMaterial _mesh 0 "/Game/LevelPrototyping/Materials/M_DamageFlash.M_DamageFlash")
  (Rendering|Material|SetMaterial _mesh 1 "/Game/LevelPrototyping/Materials/M_DamageFlash.M_DamageFlash")
  (Utilities|FlowControl|Delay 0.2)
  (Rendering|Material|SetMaterial _mesh 0 "/Game/Characters/Mannequins/Materials/Instances/Quinn/MI_Quinn_01.MI_Quinn_01")
  (Rendering|Material|SetMaterial _mesh 1 "/Game/Characters/Mannequins/Materials/Instances/Quinn/MI_Quinn_02.MI_Quinn_02"))

(event EventTick
  (params (DeltaSeconds :type Float%20%28single-precision%29))
  (bind _overlappingactors (Collision|GetOverlappingActors "/Script/Engine.TriggerSphere" :!class /Script/Engine.Actor))
  (bind _returnvalue (Utilities|Array|Length _overlappingactors))
  ;[0.15 0.15 0.15 0.5] Gravity Control
  (if (== _returnvalue 0)
    (Class|CharacterMovementComponent|SetGravityDirection (Variables|Character|GetCharacterMovement) (Math|Vector|MakeVector 0.0 0.0 0.0))
    (else
      (Class|CharacterMovementComponent|SetGravityDirection (Variables|Character|GetCharacterMovement) (Math|Vector|Normalize (- (Transformation|GetActorLocation (Utilities|Array|Get(acopy) _overlappingactors (- _returnvalue 1))) (Transformation|GetActorLocation)))))))

(fn ConstructionScript)